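; BP_SphereSpawner is an actor that periodically spawns BP_SmallSphere actors at random points around itself.
; On BeginPlay it starts a looping timer at SpawnTime intervals that fires the spawn event.
; Each spawn uses a random rotation and a location from GetRandomPointInSphereRadius, which offsets the spawner's position along a random direction by a random distance up to SpawnRadius.
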(event Custom|SpawnSmallSphere
  ;[0.15 0.15 0.15 0.5] Spawn small spheres at random locations with timer
  (Game|SpawnActorfromClass "/Game/Blueprints/SmallSphere/BP_SmallSphere.BP_SmallSphere_C" (Math|Transform|MakeTransform (CallFunction|GetRandomPointinSphereRadius) (Math|Random|RandomRotator false) "1.000000,1.000000,1.000000") "Undefined" "MultiplyWithRoot" 0 0))

(event EventBeginPlay
  ;[0.15 0.15 0.15 0.5] Spawn small spheres at random locations with timer
  (Utilities|Time|SetTimerbyEvent (delegate Custom|SpawnSmallSphere) (Variables|SphereSpawner|GetSpawnTime) true))

(fn ConstructionScript)

(fn GetRandomPointinSphereRadius
  (return (+ (Transformation|GetActorLocation) (* (Math|Vector|GetForwardVector (Math|Random|RandomRotator false)) (Math|Random|RandomFloatinRange 0.0 (Variables|SphereSpawner|GetSpawnRadius))))))